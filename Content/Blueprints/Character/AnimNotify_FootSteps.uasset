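; Animation notify that plays character footstep sounds and surface-matched particle effects.
; It spawns an attached sound at half volume when the BP_Character owner is crouched, passing the footstep mode as an integer parameter.
; A short vertical trace at the mesh origin finds the physical surface, which sets the sound's surface parameter and selects the Niagara system spawned at the configured bone.
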(fn ReceivedNotify
  (params (MeshComp :type Skeletal%20Mesh%20Component%20Object%20Reference) (Animation :type Anim%20Sequence%20Base%20Object%20Reference))
  (bind _sound (Variables|Default|GetSound))
  (bind _returnvalue (Transformation|GetWorldLocation MeshComp))
  (Utilities|IsValid MeshComp
    (:Is%20Valid
      (Utilities|IsValid Animation
        (:Is%20Valid
          (Utilities|IsValid _sound
            (:Is%20Valid
              (bind _returnvalue_2 (Audio|SpawnSoundAttached _sound MeshComp (Variables|Default|GetAttach%20Point%20Name) "0, 0, 0" "0, 0, 0" "KeepWorldPosition" false (select (Variables|/Script/Engine.Character|GetbIsCrouched (.AsBP%20Character (Utilities|Casting|CastToBP_Character (Components|GetOwner MeshComp)))) 0.5 1.0) (Variables|Default|GetPitch%20Multiplier) 0.0 0 0))
              (Utilities|IsValid _returnvalue_2
                (:Is%20Valid
                  (Effects|Components|ParticleSystem|SetIntParameter _returnvalue_2 "FootStepModes" (Math|Conversions|ToInteger(Byte) (Variables|Default|GetFootStepsModes)))
                  (bind (_outhit _returnvalue_3) (Collision|LineTraceByChannel (+ _returnvalue "0, 0,15.000000") (+ _returnvalue "0, 0,-15.000000") "TraceTypeQuery1" false 0 "None"))
                  (if _returnvalue_3
                    (Effects|Components|ParticleSystem|SetIntParameter _returnvalue_2 "Surfaces" (Math|Conversions|ToInteger(Byte) (Collision|GetSurfaceType _outhit)))
                    (Niagara|SpawnSystematLocation (Utilities|Select :Index (Collision|GetSurfaceType _outhit) :SurfaceType_Default "/Game/A_Surface_Footstep/Niagara_FX/ParticleSystems/PSN_General2_Surface.PSN_General2_Surface" :SurfaceType1 0 :SurfaceType2 "/Game/A_Surface_Footstep/Niagara_FX/ParticleSystems/PSN_Sand_Surface.PSN_Sand_Surface" :SurfaceType3 "/Game/A_Surface_Footstep/Niagara_FX/ParticleSystems/PSN_Dirt_Surface.PSN_Dirt_Surface" :SurfaceType4 "/Game/A_Surface_Footstep/Niagara_FX/ParticleSystems/PSN_WaterLight_Surface.PSN_WaterLight_Surface" :SurfaceType5 "/Game/A_Surface_Footstep/Niagara_FX/ParticleSystems/PSN_Grass_Surface.PSN_Grass_Surface" :SurfaceType6 0 :SurfaceType7 "/Game/A_Surface_Footstep/Niagara_FX/ParticleSystems/PSN_Mud_Surface.PSN_Mud_Surface" :SurfaceType8 "/Game/A_Surface_Footstep/Niagara_FX/ParticleSystems/PSN_Gravel_Surface.PSN_Gravel_Surface" :SurfaceType9 0 :SurfaceType10 "/Game/A_Surface_Footstep/Niagara_FX/ParticleSystems/PSN_SnowLight_Surface.PSN_SnowLight_Surface") (Transformation|GetSocketLocation MeshComp (Variables|Default|GetBoneNames)))
                    (return true)))
                (:Is%20Not%20Valid
                  (return false))))))))))